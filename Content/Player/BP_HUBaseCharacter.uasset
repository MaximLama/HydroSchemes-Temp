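; Player base character Blueprint that owns and controls the inventory screen.
; On BeginPlay it creates WBP_Inventory for player controller 0, adds it to the viewport and keeps it hidden.
; Tab drives a FlipFlop that shows or hides the widget, switching input mode and mouse cursor to match.
; The AddtoUIInventory event forwards inventory elements to the widget's list.
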(event EventBeginPlay
  (bind _returnvalue (UserInterface|CreateWidget "/Game/UI/WBP_Inventory.WBP_Inventory_C" (Game|GetPlayerController 0)))
  (bind _output_get (Variables|Default|SetInventoryWidget _returnvalue))
  (UserInterface|Viewport|AddtoViewport _output_get 0)
  (Widget|SetVisibility _output_get "Hidden"))

(event Collision|EventActorBeginOverlap
  (params (OtherActor :type Actor%20Object%20Reference)))

(event EventTick
  (params (DeltaSeconds :type Float%20%28single-precision%29)))

(event EventAddtoUIInventory
  (params (InventoryElement :type Inventory%20Element%20Structure))
  (Default|AddItemtoListUI (Variables|Default|GetInventoryWidget) InventoryElement))

(event Input|KeyboardEvents|Tab
  (params (Key :type Key%20Structure :default "None"))
  (bind _returnvalue (Game|GetPlayerController 0))
  (:Pressed
    (Utilities|FlowControl|FlipFlop
      (:A
        (bind _inventorywidget (Variables|Default|GetInventoryWidget)
          (:then
            (Widget|SetVisibility _inventorywidget "Visible")
            (Input|SetInputModeGameandUI _returnvalue _inventorywidget "DoNotLock" true false)
            (Variables|/Script/Engine.PlayerController|SetbShowMouseCursor _returnvalue true))
          (:else)))
      (:B
        (bind _inventorywidget_2 (Variables|Default|GetInventoryWidget)
          (:then
            (Widget|SetVisibility _inventorywidget_2 "Hidden")
            (Input|SetInputModeGameOnly _returnvalue false)
            (Variables|/Script/Engine.PlayerController|SetbShowMouseCursor _returnvalue false))
          (:else))))))

(fn ConstructionScript)